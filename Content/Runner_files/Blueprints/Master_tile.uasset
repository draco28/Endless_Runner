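; Master tile for an endless runner that spawns its own obstacles and extends the track as the player advances.
; On BeginPlay, nested random rolls may spawn obstacles across three lanes, with pipes in lanes 1 and 2 and no class set for lane 0.
; When the character overlaps the Box, the game mode spawns another tile and resets CurrentPoint, walk speed rises within a clamp, and the tile self-destroys after a short delay.
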(event OnComponentBeginOverlap(Box)
  (params (OverlappedComponent :type Primitive%20Component%20Object%20Reference) (OtherActor :type Actor%20Object%20Reference) (OtherComp :type Primitive%20Component%20Object%20Reference) (OtherBodyIndex :type Integer) (bFromSweep :type Boolean) (SweepResult :type Hit%20Result%20Structure%20%28by%20ref%29))
  (Utilities|Casting|CastToThirdPersonCharacter OtherActor)
  (bind _asthird_person_game_mode (Utilities|Casting|CastToThirdPersonGameMode (Game|GetGameMode)))
  (Default|SpawnTile _asthird_person_game_mode)
  (bind _asthird_person_game_mode_2 (Utilities|Casting|CastToThirdPersonGameMode (Game|GetGameMode)))
  (bind _output_get (Variables|/Game/ThirdPersonBP/Blueprints/ThirdPersonGameMode.ThirdPersonGameMode_C|SetCurrent_point _asthird_person_game_mode_2 0))
  (Development|PrintString (Utilities|String|ToString(Integer) _output_get))
  ;[1 1 1] speed adjustment
  (bind _asthird_person_character (Utilities|Casting|CastToThirdPersonCharacter (Game|GetPlayerCharacter 0)))
  (Variables|/Script/Engine.CharacterMovementComponent|SetMaxWalkSpeed (Variables|/Script/Engine.Character|GetCharacterMovement _asthird_person_character) (Math|Float|Clamp(Float) (* (Variables|/Script/Engine.CharacterMovementComponent|GetMaxWalkSpeed (Variables|/Script/Engine.Character|GetCharacterMovement _asthird_person_character)) 1.06) 6e+02 1.5e+03))
  ;[1 1 1] destroying tiles
  (Utilities|FlowControl|Delay 0.5)
  (Actor|DestroyActor))

(event EventBeginPlay
  ;[1 1 1] obsticles
  (CallFunction|SpawnObsticles))

(event Collision|EventActorBeginOverlap
  (params (OtherActor :type Actor%20Object%20Reference)))

(event EventTick
  (params (DeltaSeconds :type Float%20%28single-precision%29)))

(fn ConstructionScript)

(fn SpawnObsticles
  ;[1 1 1] lane 0
  (switch int (Math|Random|RandomIntegerinRange 0 3)
    (:3
      (Game|SpawnActorfromClass "/Game/Runner_files/Blueprints/Obsticles_pipe.Obsticles_pipe_C" (Transformation|GetWorldTransform (Variables|Default|Getlane0)) "Undefined" 0 0)
      ;[1 1 1] lane 1
      (switch int (Math|Random|RandomIntegerinRange 0 2)
        (:1
          (Game|SpawnActorfromClass "/Game/Runner_files/Blueprints/Obsticles_pipe.Obsticles_pipe_C" (Transformation|GetWorldTransform (Variables|Default|Getlane1)) "Undefined" 0 0)
          ;[1 1 1] lane 2
          (switch int (Math|Random|RandomIntegerinRange 0 1)
            (:1
              (Game|SpawnActorfromClass "/Game/Runner_files/Blueprints/Obsticles_pipe.Obsticles_pipe_C" (Transformation|GetWorldTransform (Variables|Default|Getlane2)) "Undefined" 0 0))))))))